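; Level manager that tracks target score and stages the world-change sequence for the game.
; On BeginPlay it pre-spawns a hidden, layer-tagged tracking-object pool, counts layered targets for the 3D score text, and test-fires the all-targets event after a delay.
; Changeworld masks sky and landscape parameter-collection changes with a monolith laser, non-VR camera shake and fades.
; The all-targets event plays audio and sets a flag; reaching the total and Game_Complete trigger nothing.
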(event Custom|Change%20world
  (bind _returnvalue (Game|GetPlayerCameraManager 0))
  (bind _sky_sphere (Variables|Default|GetSky_Sphere))
  (bind _monolite (Variables|Default|GetMonolite))
  (Default|CreateLaser _monolite)
  (Utilities|FlowControl|Delay 4.0)
  ;[0.6655 1 0.6641] Camera shake and fade
  (if (Variables|/Game/Characters/BP_Character.BP_Character_C|GetPlaying_VR? (Variables|Default|GetBP%20Character))
    _
    (else
      (CameraShakes|StartCameraShake _returnvalue "/Game/UI/BP_Camera-Shake.BP_Camera-Shake_C" 5.0 "CameraLocal" "0, 0, 0")))
  (CameraFades|StartCameraFade :self _returnvalue :ToAlpha 1.0 :Duration 0.5 :bHoldWhenFinished true)
  (Utilities|FlowControl|Delay 1.0)
  ;[1 0.9092 0.4678] World aspect change
  (Default|UpdateLight _sky_sphere)
  (Default|ChangeSkyColor _sky_sphere "(R=0.000000,G=0.004777,B=0.004777,A=1.000000)" "(R=0.000000,G=0.201556,B=0.171441,A=1.000000)" "(R=0.423268,G=0.973446,B=0.973446,A=1.000000)" "(R=0.423268,G=0.973446,B=0.973446,A=1.000000)" true)
  (Rendering|Material|SetScalarParameterValue "/Game/Landscape/Materials/MPC_Landscape.MPC_Landscape" (Variables|Default|GetMPC%20Param%20Name) 1.0 :!class /Script/Engine.KismetMaterialLibrary)
  (Default|DestroyLaser _monolite)
  (Utilities|FlowControl|Delay 0.5)
  (CameraFades|StartCameraFade :self _returnvalue :FromAlpha 1.0 :Duration 0.5 :bHoldWhenFinished true))

(event Custom|Game_Complete)

(event Custom|Increase%20Score
  (bind _result (Math|Integer|IncrementInt (Variables|Default|GetNumber%20Targets%20Hitted))
    (:%20%20
      (CallFunction|SetScoreText)
      ;[1 1 1] If all targets hitted launch event
      (if (== _result (Variables|Default|GetNumber%20Targets%20Total))
        _))))

(event Custom|All_Targets_Hitted
  (Audio|Components|Audio|Play (Variables|Default|GetAudio) 0.0)
  (Variables|Default|SetAll%20targets%20hitted true))

(event EventBeginPlay
  (CallFunction|CreateTrackingObjectPool)
  (CallFunction|SetScore)
  (bind _asbp_character (Utilities|Casting|CastToBP_Character (Game|Player|GetPlayerPawn 0)))
  (Variables|Default|SetBP%20Character _asbp_character)
  ;[1 1 1] Test
  (Utilities|FlowControl|Delay 3.0)
  (CallFunction|AllTargetsHitted))

(event Collision|EventActorBeginOverlap
  (params (OtherActor :type Actor%20Object%20Reference)))

(event EventTick
  (params (DeltaSeconds :type Float%20%28single-precision%29)))

(fn ConstructionScript)

(fn CreateTrackingObjectPool
  (for _index (range 0 (Variables|Default|GetNumber%20Tracking%20Objects))
    (bind _returnvalue (Game|SpawnActorfromClass (Variables|Default|GetTracking%20Object%20Class) (Math|Transform|MakeTransform "0, 0, 0" "0,180.000000, 0" "1,1,1") "Undefined" 0 0))
    (Class|LayersBlueprintLibrary|AddActortoLayer _returnvalue (Variables|Default|GetTracking%20Objects%20Pool%20Layer))
    (Rendering|SetActorHiddenInGame _returnvalue true)))

(fn SetScore
  ;[1 1 1] Get targets
  (bind _returnvalue (Class|LayersBlueprintLibrary|GetActors (Variables|Default|GetTarget%20Objects%20Layer)))
  (Variables|Default|SetNumber%20Targets%20Total (Utilities|Array|Length _returnvalue))
  (CallFunction|SetScoreText)
  (for _array_element _returnvalue
    (Utilities|Casting|CastToBP_Target _array_element)))

(fn SetScoreText
  (Class|Text3DComponent|SetText (Variables|/Script/Text3D.Text3DActor|GetText3DComponent (Variables|Default|GetScore%203D%20Text)) (Utilities|Text|FormatText (LocalVariables|GetFormat%20Text) (Utilities|Text|ToText(Integer) (Variables|Default|GetNumber%20Targets%20Hitted)) (Utilities|Text|ToText(Integer) (Variables|Default|GetNumber%20Targets%20Total)))))