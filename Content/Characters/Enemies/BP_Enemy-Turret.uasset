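; Turret enemy, a child of an enemy base, that detects the player with an overlap sphere and attacks with a Niagara laser beam.
; On detection in a specific state, a timeline sweeps the beam end to the player; losing the player switches the laser off.
; Attack line-traces toward the player, snaps the beam to the hit and calls the parent attack only if the player character is hit.
; Fracturing its destructible component destroys the turret.
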(event OnComponentBeginOverlap(Sphere)
  (params (OverlappedComponent :type Primitive%20Component%20Object%20Reference) (OtherActor :type Actor%20Object%20Reference) (OtherComp :type Primitive%20Component%20Object%20Reference) (OtherBodyIndex :type Integer) (bFromSweep :type Boolean) (SweepResult :type Hit%20Result%20Structure%20%28by%20ref%29))
  ;[1 1 1] Check if player
  (bind _asbp_character (Utilities|Casting|CastToBP_Character OtherActor))
  (Variables|Default|SetPlayer _asbp_character)
  (CallFunction|OnDetectPlayer))

(event OnComponentEndOverlap(Sphere)
  (params (OverlappedComponent :type Primitive%20Component%20Object%20Reference) (OtherActor :type Actor%20Object%20Reference) (OtherComp :type Primitive%20Component%20Object%20Reference) (OtherBodyIndex :type Integer))
  ;[1 1 1] Check if player
  (if (== OtherActor (Variables|Default|GetPlayer))
    (CallFunction|OnLostPlayer)))

(event OnComponentFracture(Destructible)
  (params (HitPoint :type Vector%20%28by%20ref%29 :default "0, 0, 0") (HitDirection :type Vector%20%28by%20ref%29 :default "0, 0, 0"))
  (bind _ns_laser (Variables|Default|GetNS_Laser))
  (if (Components|Activation|IsActive _ns_laser)
    (Components|Activation|Deactivate _ns_laser))
  (Actor|DestroyActor))

(event EventBeginPlay
  (Variables|Default|SetState "NewEnumerator2"))

(event Collision|EventActorBeginOverlap
  (params (OtherActor :type Actor%20Object%20Reference)))

(event EventTick
  (params (DeltaSeconds :type Float%20%28single-precision%29)))

(event EventOnDetectPlayer
  (bind _returnvalue (Transformation|GetActorLocation))
  (|CallParentFunction)
  (if (Utilities|Enum|Equal(Enum) "NewEnumerator3" (Variables|Default|GetState))
    ;[1 1 1] Laser Beam interpolation
    (Components|Activation|Activate (Variables|Default|GetNS_Laser) false)
    (bind _alpha (Timeline|Interpolate%20positions PlayFromStart)
      (:Update
        (Effects|Components|ParticleSystem|SetVectorParameter (Variables|Default|GetNS_Laser) "Beam End" (Math|Vector|Lerp(Vector) (Math|Vector|MakeVector (.x _returnvalue) (.y _returnvalue) (+ (.z _returnvalue) 49.0)) (Transformation|GetActorLocation (Variables|Default|GetPlayer)) _alpha))))))

(event EventOnLostPlayer
  (|CallParentFunction)
  (Components|Activation|Deactivate (Variables|Default|GetNS_Laser)))

(fn ConstructionScript
  (Variables|Default|SetDamage (Variables|Default|GetConcrete_Damage)))

(fn Attack
  (bind _player (Variables|Default|GetPlayer))
  (if true
    (Utilities|IsValid _player
      (:Is%20Valid
        (bind _outhit (Collision|LineTraceByChannel (Transformation|GetActorLocation) (Transformation|GetActorLocation _player) "TraceTypeQuery6" false 0 "None"))
        (Effects|Components|ParticleSystem|SetVectorParameter (Variables|Default|GetNS_Laser) "Beam End" (.location _outhit))
        ;[1 1 1] Trackig collide with player
        (Utilities|Casting|CastToBP_Character (.hitactor _outhit))
        (|CallParentFunction)))))