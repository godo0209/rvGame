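; BP_Enemy-Spawn is an unfinished enemy spawn point that caches GS_Base on BeginPlay.
; TrySpawn compares its own count and the GameState's living-enemy count against their limits, but the passing branch does nothing.
; The SpawnActor node for EnemyClass and the random navigable-point lookup within the Sphere radius are both unwired.
; Nothing in the shown graphs calls TrySpawn, and GetEnemyPosition is empty.
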(event EventBeginPlay
  (bind _asgs_base (Utilities|Casting|CastToGS_Base (Game|GetGameState)))
  (Variables|Default|SetGame%20State _asgs_base))

(event Collision|EventActorBeginOverlap
  (params (OtherActor :type Actor%20Object%20Reference)))

(event EventTick
  (params (DeltaSeconds :type Float%20%28single-precision%29)))

(fn ConstructionScript)

(fn TrySpawn
  (bind _game_state (Variables|Default|GetGame%20State))
  (if (and (< (Variables|Default|GetCurrent%20Num%20Enemies) (Variables|Default|GetNum%20Enemies%20To%20Spawn)) (< (Variables|/Game/Core/GS_Base.GS_Base_C|GetCurrent%20Enemies%20Alive _game_state) (Variables|/Game/Core/GS_Base.GS_Base_C|GetMax%20Enemies%20Alive _game_state)))
    _))

(fn GetEnemyPosition)