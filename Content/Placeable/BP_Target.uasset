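; BP_Target is a placeable target that awards score when an active BP_Arrow hits it.
; Its Sphere overlap event casts to BP_Arrow, increases score through LvlFunctions, sets IsColliding to block repeat hits and plays audio.
; After a short delay it destroys the TargetHolder, if valid, and then itself.
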(event OnComponentBeginOverlap(Sphere)
  (params (OverlappedComponent :type Primitive%20Component%20Object%20Reference) (OtherActor :type Actor%20Object%20Reference) (OtherComp :type Primitive%20Component%20Object%20Reference) (OtherBodyIndex :type Integer) (bFromSweep :type Boolean) (SweepResult :type Hit%20Result%20Structure%20%28by%20ref%29))
  (bind _target_holder (Variables|Default|GetTarget%20Holder))
  (if (not (Variables|Default|GetIs%20Colliding?))
    ;[1 1 1] To know if the collision was with an arrow and is active
    (bind _asbp_arrow (Utilities|Casting|CastToBP_Arrow OtherActor))
    (if (Variables|/Game/Placeable/Weapon_Blueprints/BP_Arrow.BP_Arrow_C|GetIs%20Active? _asbp_arrow)
      (Default|IncreaseScore (Variables|Default|GetLvl_Functions))
      (Variables|Default|SetIs%20Colliding? true)
      (Audio|Components|Audio|Play (Variables|Default|GetAudio) 0.0)
      ;[1 1 1] Delay For the explosion (niagara) and check for holder
      (Utilities|FlowControl|Delay 0.15)
      (Utilities|IsValid _target_holder
        (:Is%20Valid
          (Actor|DestroyActor _target_holder))
        (:Is%20Not%20Valid
          _))
      (Actor|DestroyActor))))

(event EventBeginPlay)

(event Collision|EventActorBeginOverlap
  (params (OtherActor :type Actor%20Object%20Reference)))

(event EventTick
  (params (DeltaSeconds :type Float%20%28single-precision%29)))

(fn ConstructionScript)