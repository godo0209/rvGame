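; BP_Menu is an in-world menu, hidden on construction, whose options are selected by hitting them with active arrows.
; Show_Menu toggles visibility and moves it to a given spawn point, rotated toward the player pawn.
; Leaving the Sphere trigger repeats that placement.
; Both option spheres share one guarded hit check: Continue hides the menu, while Out fades the camera and audio, then quits the game.
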(event OnComponentBeginOverlap(SphereContinue)
  (params (OverlappedComponent :type Primitive%20Component%20Object%20Reference) (OtherActor :type Actor%20Object%20Reference) (OtherComp :type Primitive%20Component%20Object%20Reference) (OtherBodyIndex :type Integer) (bFromSweep :type Boolean) (SweepResult :type Hit%20Result%20Structure%20%28by%20ref%29))
  (Variables|Default|SetSphere%20Collider 0)
  (Variables|Default|SetCollider%20Actor OtherActor)
  (if (not (Variables|Default|GetIs%20Colliding?))
    ;[1 1 1] To know if the collision was with an arrow and is active
    (bind _asbp_arrow (Utilities|Casting|CastToBP_Arrow (Variables|Default|GetCollider%20Actor)))
    (if (Variables|/Game/Placeable/Weapon_Blueprints/BP_Arrow.BP_Arrow_C|GetIs%20Active? _asbp_arrow)
      (Variables|Default|SetIs%20Colliding? true)
      (switch int (Variables|Default|GetSphere%20Collider)
        (:0
          ;[1 1 1] Continue
          (Rendering|SetActorHiddenInGame true)
          (Utilities|FlowControl|Delay 0.1)
          (Variables|Default|SetIs%20Colliding? false))
        (:1
          ;[1 1 1] End Game
          (CameraFades|StartCameraFade :self (Game|GetPlayerCameraManager 0) :ToAlpha 1.0 :Duration 0.5 :bShouldFadeAudio true :bHoldWhenFinished true)
          (Utilities|FlowControl|Delay 1.0)
          (Game|QuitGame 0 "Quit" false))))))

(event OnComponentBeginOverlap(SphereOut)
  (params (OverlappedComponent :type Primitive%20Component%20Object%20Reference) (OtherActor :type Actor%20Object%20Reference) (OtherComp :type Primitive%20Component%20Object%20Reference) (OtherBodyIndex :type Integer) (bFromSweep :type Boolean) (SweepResult :type Hit%20Result%20Structure%20%28by%20ref%29))
  (Variables|Default|SetSphere%20Collider 1)
  (Variables|Default|SetCollider%20Actor OtherActor)
  (if (not (Variables|Default|GetIs%20Colliding?))
    ;[1 1 1] To know if the collision was with an arrow and is active
    (bind _asbp_arrow (Utilities|Casting|CastToBP_Arrow (Variables|Default|GetCollider%20Actor)))
    (if (Variables|/Game/Placeable/Weapon_Blueprints/BP_Arrow.BP_Arrow_C|GetIs%20Active? _asbp_arrow)
      (Variables|Default|SetIs%20Colliding? true)
      (switch int (Variables|Default|GetSphere%20Collider)
        (:0
          ;[1 1 1] Continue
          (Rendering|SetActorHiddenInGame true)
          (Utilities|FlowControl|Delay 0.1)
          (Variables|Default|SetIs%20Colliding? false))
        (:1
          ;[1 1 1] End Game
          (CameraFades|StartCameraFade :self (Game|GetPlayerCameraManager 0) :ToAlpha 1.0 :Duration 0.5 :bShouldFadeAudio true :bHoldWhenFinished true)
          (Utilities|FlowControl|Delay 1.0)
          (Game|QuitGame 0 "Quit" false))))))

(event OnComponentEndOverlap(Sphere)
  (params (OverlappedComponent :type Primitive%20Component%20Object%20Reference) (OtherActor :type Actor%20Object%20Reference) (OtherComp :type Primitive%20Component%20Object%20Reference) (OtherBodyIndex :type Integer))
  (bind _spawn_point (Variables|Default|GetSpawn%20Point))
  (bind _returnvalue (Transformation|GetWorldLocation _spawn_point))
  (Utilities|IsValid _spawn_point
    (:Is%20Valid
      (Transformation|SetActorLocationAndRotation _returnvalue (Math|Rotator|FindLookatRotation _returnvalue (Transformation|GetActorLocation (Game|Player|GetPlayerPawn 0)))))))

(event Custom|Show_Menu
  (params (Spawn%20Point :type Scene%20Component%20Object%20Reference))
  (Variables|Default|SetSpawn%20Point Spawn%20Point)
  (Rendering|SetActorHiddenInGame (not (Variables|Rendering|GetbHidden)))
  (Transformation|SetActorLocationAndRotation (Transformation|GetWorldLocation (Variables|Default|GetSpawn%20Point)) (Math|Rotator|FindLookatRotation (Transformation|GetWorldLocation (Variables|Default|GetSpawn%20Point)) (Transformation|GetActorLocation (Game|Player|GetPlayerPawn 0)))))

(event EventBeginPlay)

(event Collision|EventActorBeginOverlap
  (params (OtherActor :type Actor%20Object%20Reference)))

(event EventTick
  (params (DeltaSeconds :type Float%20%28single-precision%29)))

(fn ConstructionScript
  (Rendering|SetActorHiddenInGame true))