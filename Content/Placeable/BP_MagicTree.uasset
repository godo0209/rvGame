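; BP_MagicTree is a placeable actor that shows a Niagara laser beam and a rotating "sun" mesh.
; CreateLaser activates the beam, raises its end point skyward with one timeline, then expands its sphere size with a second.
; DestroyLaser deactivates the beam, unhides the mesh and enables its constant rotation on Tick.
; The construction script sets the beam's initial end just above the actor.
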(event Custom|Create%20Laser
  (bind _returnvalue (Transformation|GetActorLocation))
  (bind _niagara (Variables|Default|GetNiagara))
  (Components|Activation|Activate _niagara false)
  (bind _off_set_z (Timeline|Increase%20offset%20z Play)
    (:Update
      (Effects|Components|ParticleSystem|SetVectorParameter _niagara "Beam End" (Math|Vector|MakeVector (.x _returnvalue) (.y _returnvalue) (+ (Math|Float|Lerp 205.0 3e+03 _off_set_z) (.z _returnvalue)))))
    (:Finished
      (bind _sphere_expand (Timeline|Timeline_0 Play)
        (:Update
          (Effects|Components|ParticleSystem|SetFloatParameter _niagara "Sphere Rand Max Size" (Math|Float|Lerp 4e+01 4e+02 _sphere_expand))
          (Effects|Components|ParticleSystem|SetFloatParameter _niagara "Sphere Rand Min Size" (Math|Float|Lerp 4e+01 4e+02 _sphere_expand)))))))

(event Custom|Destroy%20Laser
  (Components|Activation|Deactivate (Variables|Default|GetNiagara))
  (Development|SetHiddeninGame (Variables|Default|GetStaticMesh1) false false)
  (Variables|Default|SetRotate%20Sun true))

(event EventBeginPlay)

(event Collision|EventActorBeginOverlap
  (params (OtherActor :type Actor%20Object%20Reference)))

(event EventTick
  (params (DeltaSeconds :type Float%20%28single-precision%29))
  (if (Variables|Default|GetRotate%20Sun)
    (Transformation|AddLocalRotation (Variables|Default|GetStaticMesh1) (Variables|Default|GetRotation%20Vel) false false)))

(fn ConstructionScript
  (bind _returnvalue (Transformation|GetActorLocation))
  (Effects|Components|ParticleSystem|SetVectorParameter (Variables|Default|GetNiagara) "Beam End" (Math|Vector|MakeVector (.x _returnvalue) (.y _returnvalue) (+ (.z _returnvalue) 205.0))))