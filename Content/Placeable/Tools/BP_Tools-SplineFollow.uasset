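; Placeable spline tool that lines a path with instanced static meshes, built entirely in the construction script.
; Each instanced mesh component under the spline takes its mesh from MeshesToInstance by index, with optional X/Y scale negation through FlipMeshes.
; Spacing comes from the first mesh's X bounds plus an offset.
; Each step adds an instance to a randomly chosen child component, oriented toward the next position.
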(event EventBeginPlay)

(event Collision|EventActorBeginOverlap
  (params (OtherActor :type Actor%20Object%20Reference)))

(event EventTick
  (params (DeltaSeconds :type Float%20%28single-precision%29)))

(fn ConstructionScript
  (bind _meshes_to_instance (Variables|Default|GetMeshes_To_Instance))
  (bind _output (Utilities|Array|Get(acopy) _meshes_to_instance))
  (bind _returnvalue (StaticMesh|GetBoundingBox _output))
  (CallFunction|SetStaticMeshes)
  (bind _output_get (Variables|Default|SetSpacing (+ (.x (- (.max _returnvalue) (.min _returnvalue))) (Variables|Default|GetOffset))))
  (bind _output_get_2 (LocalVariables|SetNum_Instances (Math|Float|Floor (/ (Spline|GetSplineLength (Variables|Default|GetSpline)) _output_get))))
  (for _index (range 0 _output_get_2)
    (bind _asinstanced_static_mesh_component (Utilities|Casting|CastToInstancedStaticMeshComponent (.OutItem (Utilities|Array|Random (Components|GetChildrenComponents (Variables|Default|GetSpline) false)))))
    (Components|InstancedStaticMesh|AddInstance _asinstanced_static_mesh_component (Math|Transform|MakeTransform (Utilities|GetInstanceLocationbyIndex _index) (Math|Rotator|MakeRotfromX (- (Utilities|GetInstanceLocationbyIndex (+ _index 1)) (Utilities|GetInstanceLocationbyIndex _index)))))))

(fn SetStaticMeshes
  (for (_array_element _array_index) (Components|GetChildrenComponents (Variables|Default|GetSpline) false)
    (bind _asinstanced_static_mesh_component (Utilities|Casting|CastToInstancedStaticMeshComponent _array_element))
    (Components|StaticMesh|SetStaticMesh _asinstanced_static_mesh_component (Utilities|Array|Get(acopy) (Variables|Default|GetMeshes_To_Instance) _array_index))
    (if (Variables|Default|GetFlip_Meshes?)
      (Transformation|SetRelativeScale3D _asinstanced_static_mesh_component (Math|Vector|MakeVector (* -1.0 (.x (Transformation|GetWorldScale _asinstanced_static_mesh_component))) (* -1.0 (.y (Transformation|GetWorldScale _asinstanced_static_mesh_component))) (.z (Transformation|GetWorldScale _asinstanced_static_mesh_component)))))))