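; Placeable spline tool that lines a spline with deformed meshes picked at random from MeshesToInstance.
; The construction script derives spacing from the first mesh's X bounds plus Offset, then adds spline mesh components along the spline's length.
; Segment endpoints and tangents come from an index-based helper.
; SetStaticMeshes, which assigns and optionally flips child instanced meshes, is never called here.
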(event EventBeginPlay)

(event Collision|EventActorBeginOverlap
  (params (OtherActor :type Actor%20Object%20Reference)))

(event EventTick
  (params (DeltaSeconds :type Float%20%28single-precision%29)))

(fn ConstructionScript
  (bind _meshes_to_instance (Variables|Default|GetMeshes_To_Instance))
  (bind _output (Utilities|Array|Get(acopy) _meshes_to_instance))
  (bind _returnvalue (StaticMesh|GetBoundingBox _output))
  (bind _output_get (Variables|Default|SetSpacing (+ (.x (+ (Math|Vector|VectorGetAbs (.min _returnvalue)) (Math|Vector|VectorGetAbs (.max _returnvalue)))) (Variables|Default|GetOffset))))
  (bind _output_get_2 (LocalVariables|SetNum_Instances (Math|Float|Floor (/ (Spline|GetSplineLength (Variables|Default|GetSpline)) _output_get))))
  (for _index (range 0 _output_get_2)
    (bind _returnvalue_2 (AddComponent|AddSplineMeshComponent false))
    (SplineMesh|SetForwardAxis _returnvalue_2 "X" true)
    (Components|StaticMesh|SetStaticMesh _returnvalue_2 (.OutItem (Utilities|Array|Random (Variables|Default|GetMeshes_To_Instance))))
    (SplineMesh|SetStartandEnd _returnvalue_2 (.Location (Utilities|GetInstanceLocationandTangentbyIndex _index)) (.Tangent (Utilities|GetInstanceLocationandTangentbyIndex _index)) (.Location (Utilities|GetInstanceLocationandTangentbyIndex (+ _index 1))) (.Tangent (Utilities|GetInstanceLocationandTangentbyIndex (+ _index 1))) true :!class /Script/Engine.SplineMeshComponent)))

(fn SetStaticMeshes
  (for (_array_element _array_index) (Components|GetChildrenComponents (Variables|Default|GetSpline) false)
    (bind _asinstanced_static_mesh_component (Utilities|Casting|CastToInstancedStaticMeshComponent _array_element))
    (Components|StaticMesh|SetStaticMesh _asinstanced_static_mesh_component (Utilities|Array|Get(acopy) (Variables|Default|GetMeshes_To_Instance) _array_index))
    ;[1 1 1] Flip meshes
    (if (Variables|Default|GetFlip_Meshes?)
      (Transformation|SetRelativeScale3D _asinstanced_static_mesh_component (Math|Vector|MakeVector (* -1.0 (.x (Transformation|GetWorldScale _asinstanced_static_mesh_component))) (* -1.0 (.y (Transformation|GetWorldScale _asinstanced_static_mesh_component))) (.z (Transformation|GetWorldScale _asinstanced_static_mesh_component)))))))