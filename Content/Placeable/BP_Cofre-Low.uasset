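; Interactable chest (cofre) that opens, spawns a weapon at its location, then fades out and destroys itself.
; CanInteract and CannotInteract fade the input prompt in or out; they and Interact act only while HiddenInActor is invalid.
; Interact triggers the opening through ABP_Cofre, while a timeline fades chest and prompt via dynamic materials cached at BeginPlay.
; A helper, uncalled here, sets chest desaturation from player distance between two sphere radii.
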(event EventBeginPlay
  ;[1 0.9436 0.577] Dont show input
  (Rendering|SetVisibility (Variables|Default|GetInput_keyboard) false true)
  ;[0.2433 0.2351 1] Create dynamic Materials
  (CallFunction|CreateDynamicMat))

(event Collision|EventActorBeginOverlap
  (params (OtherActor :type Actor%20Object%20Reference)))

(event EventTick
  (params (DeltaSeconds :type Float%20%28single-precision%29)))

(event EventInteract
  (Utilities|IsValid (Variables|Default|GetHidden%20in%20actor)
    (:Is%20Not%20Valid
      ;[0.2993 1 0.5097] On interact init animation
      (Variables|Default|SetState "NewEnumerator2")
      (CallFunction|PlayAnimation)
      ;[1 0.8427 0.4836] Spawn Weapon
      (Class|BIWeapon|Spawn(Message) (Variables|Default|GetWeapon_To_Spawn) (Transformation|GetActorLocation))
      ;[0.3895 0.3571 1] Disappear particles with size
      ;;[1 1 1] Get current input Opacity
      (bind _returnvalue (Rendering|Material|GetScalarParameterValue (.Value (Utilities|Map|Find (Variables|Default|GetDynamic_Materials) (Variables|Default|GetInput%20Button%20Key))) "Opacity" :!class /Script/Engine.MaterialInstanceDynamic))
      (Variables|Default|SetInput%20Opacity%20Before%20Despawn _returnvalue)
      (bind _alfa_track (Timeline|Alpha_Material Play)
        (:Update
          ;;[1 1 1] Clamp to 1 for size
          (if (> _alfa_track 1.0)
            (Variables|Default|SetAlpha%20Material%20On%20Interact 1.0)
            (else
              (Variables|Default|SetAlpha%20Material%20On%20Interact _alfa_track)))
          ;[1 0.4579 0.4778] Disappear mesh with opacity mat
          (Rendering|Material|SetScalarParameterValue (.Value (Utilities|Map|Find (Variables|Default|GetDynamic_Materials) (Variables|Default|GetCofre%20Base%20Key))) "Opacity" _alfa_track :!class /Script/Engine.MaterialInstanceDynamic)
          (Rendering|Material|SetScalarParameterValue (.Value (Utilities|Map|Find (Variables|Default|GetDynamic_Materials) (Variables|Default|GetCofre%20Metal%20Key))) "Opacity" _alfa_track :!class /Script/Engine.MaterialInstanceDynamic)
          ;[1 0.4579 0.4778] Disappear input mesh with opacity mat (lerp)
          (Rendering|Material|SetScalarParameterValue (.Value (Utilities|Map|Find (Variables|Default|GetDynamic_Materials) (Variables|Default|GetInput%20Button%20Key))) "Opacity" (Math|Float|Lerp 0.0 (Variables|Default|GetInput%20Opacity%20Before%20Despawn) (Variables|Default|GetAlpha%20Material%20On%20Interact)) :!class /Script/Engine.MaterialInstanceDynamic)
          (Rendering|Material|SetScalarParameterValue (.Value (Utilities|Map|Find (Variables|Default|GetDynamic_Materials) (Variables|Default|GetInput%20Text%20Key))) "Opacity" (Math|Float|Lerp 0.0 (Variables|Default|GetInput%20Opacity%20Before%20Despawn) (Variables|Default|GetAlpha%20Material%20On%20Interact)) :!class /Script/Engine.MaterialInstanceDynamic))
        (:Finished
          (Variables|Default|SetState "NewEnumerator3")
          (Actor|DestroyActor))))))

(event EventCanInteract
  (Utilities|IsValid (Variables|Default|GetHidden%20in%20actor)
    (:Is%20Not%20Valid
      ;[1 1 1] On can interact = change state
      (if (Utilities|Enum|NotEqual(Enum) (Variables|Default|GetState) "NewEnumerator2")
        (Variables|Default|SetState "NewEnumerator1")
        ;[1 1 1] Start opacity animation for input (appear)
        (bind _alpha (Timeline|Input_material_appear PlayFromStart)
          (:Update
            (Rendering|Material|SetScalarParameterValue (.Value (Utilities|Map|Find (Variables|Default|GetDynamic_Materials) (Variables|Default|GetInput%20Button%20Key))) "Opacity" _alpha :!class /Script/Engine.MaterialInstanceDynamic)
            (Rendering|Material|SetScalarParameterValue (.Value (Utilities|Map|Find (Variables|Default|GetDynamic_Materials) (Variables|Default|GetInput%20Text%20Key))) "Opacity" _alpha :!class /Script/Engine.MaterialInstanceDynamic)))))))

(event EventCannotInteract
  (Utilities|IsValid (Variables|Default|GetHidden%20in%20actor)
    (:Is%20Not%20Valid
      (if (Utilities|Enum|NotEqual(Enum) (Variables|Default|GetState) "NewEnumerator2")
        (Variables|Default|SetState "NewEnumerator0")
        ;[1 1 1] Start opacity animation for input (disappear)
        (bind _alpha (Timeline|Input%20material%20disappear PlayFromStart)
          (:Update
            (Rendering|Material|SetScalarParameterValue (.Value (Utilities|Map|Find (Variables|Default|GetDynamic_Materials) (Variables|Default|GetInput%20Button%20Key))) "Opacity" _alpha :!class /Script/Engine.MaterialInstanceDynamic)
            (Rendering|Material|SetScalarParameterValue (.Value (Utilities|Map|Find (Variables|Default|GetDynamic_Materials) (Variables|Default|GetInput%20Text%20Key))) "Opacity" _alpha :!class /Script/Engine.MaterialInstanceDynamic)))))))

(fn ConstructionScript)

(fn PlayAnimation
  ;[1 1 1] Set variable for abp that change state
  (bind _asabp_cofre (Utilities|Casting|CastToABP_Cofre (Components|SkeletalMesh|GetAnimInstance (Variables|Default|GetSkeletalMesh))))
  (Variables|/Game/Placeable/Animations/ABP_Cofre.ABP_Cofre_C|SetHas_to_Open _asabp_cofre true))

(fn PlaySound)

(fn PlayInput
  (Rendering|SetVisibility (Variables|Default|GetInput_keyboard) true true))

(fn UpdateMaterial
  (bind _newparam (CallFunction|GetNormalicedPlayerDistanceF))
  (Rendering|Material|SetScalarParameterValue (.Value (Utilities|Map|Find (Variables|Default|GetDynamic_Materials) (Variables|Default|GetCofre%20Base%20Key))) "Desaturation" _newparam :!class /Script/Engine.MaterialInstanceDynamic))

(fn GetNormalicedPlayerDistanceF
  (bind _returnvalue (Game|Player|GetPlayerPawn 0))
  (bind _returnvalue_2 (Transformation|GetActorLocation))
  (bind _saze_zone_collider (Variables|Default|GetSaze_Zone_Collider))
  (bind _interactable_collider (Variables|Default|GetInteractable_Collider))
  (bind _returnvalue_3 (Components|Sphere|GetScaledSphereRadius _interactable_collider))
  (bind _returnvalue_4 (Components|Sphere|GetScaledSphereRadius _saze_zone_collider))
  (bind _returnvalue_5 (Transformation|GetActorLocation _returnvalue))
  (bind _distance (Utilities|GetNormalicedDistance _returnvalue_2 _returnvalue_5 _returnvalue_4 _returnvalue_3))
  (if (> _distance 1.0)
    (LocalVariables|SetNewLocalVar_1 1.0)
    (elif (< _distance 0.0)
      (LocalVariables|SetNewLocalVar_1 0.0)
      (else
        (LocalVariables|SetNewLocalVar_1 _distance))))
  (return (LocalVariables|GetNewLocalVar_1)))

(fn CreateDynamicMat
  (bind _input_button_key (Variables|Default|GetInput%20Button%20Key))
  (bind _dynamic_materials (Variables|Default|GetDynamic_Materials))
  (bind _cofre_base_key (Variables|Default|GetCofre%20Base%20Key))
  (bind _input_text_key (Variables|Default|GetInput%20Text%20Key))
  (bind _cofre_metal_key (Variables|Default|GetCofre%20Metal%20Key))
  ;[0.6921 1 0.6498] Cofre base Mat
  (if (not (Utilities|DoesDymMatExist _cofre_base_key))
    (bind _returnvalue (Rendering|Material|CreateDynamicMaterialInstance (Variables|Default|GetSkeletalMesh) 0 "/Game/Placeable/Materials/MI_Cofre-Base.MI_Cofre-Base" "None" :!class /Script/Engine.PrimitiveComponent))
    (Utilities|Map|Add _dynamic_materials _cofre_base_key _returnvalue)
    ;[1 0.9573 0.575] Cofre metal Mat
    (if (not (Utilities|DoesDymMatExist _cofre_metal_key))
      (bind _returnvalue_2 (Rendering|Material|CreateDynamicMaterialInstance (Variables|Default|GetSkeletalMesh) 1 "/Game/Placeable/Materials/MI_Cofre-Oro.MI_Cofre-Oro" "None" :!class /Script/Engine.PrimitiveComponent))
      (Utilities|Map|Add _dynamic_materials _cofre_metal_key _returnvalue_2)
      ;[1 0.5359 0.6058] InputButton Mat
      (if (not (Utilities|DoesDymMatExist _input_button_key))
        (bind _returnvalue_3 (Rendering|Material|CreateDynamicMaterialInstance (Variables|Default|GetInput%20button) 0 "/Game/Placeable/Materials/Inputs/MI_Inputs-Button.MI_Inputs-Button" "None" :!class /Script/Engine.PrimitiveComponent))
        (Utilities|Map|Add _dynamic_materials _input_button_key _returnvalue_3)
        ;[0.2482 0.1506 1] InputText Mat
        (if (not (Utilities|DoesDymMatExist _input_text_key))
          (bind _returnvalue_4 (Rendering|Material|CreateDynamicMaterialInstance (Variables|Default|GetInput%20text) 0 "/Game/Placeable/Materials/Inputs/MI_Inputs-Letter.MI_Inputs-Letter" "None" :!class /Script/Engine.PrimitiveComponent))
          (Utilities|Map|Add _dynamic_materials _input_text_key _returnvalue_4))))))