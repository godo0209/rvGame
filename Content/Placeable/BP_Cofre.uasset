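; BP_Cofre is an interactable chest with a skeletal mesh and firefly particles.
; CanInteract and CannotInteract switch its state, with the former lazily creating a dynamic material.
; Interact sets the open flag on the chest's anim Blueprint and plays a timeline that drives the particles' color alpha to make them disappear.
; Helpers for distance-based desaturation and particle color blending exist, but nothing in this graph calls them.
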(event EventBeginPlay
  ;[1 1 1] Init particle color
  (Effects|Components|ParticleSystem|SetColorParameter (Variables|Default|GetParticleSystem) "Fireflies_Color" (Variables|Default|GetParticle_Init_Color)))

(event Collision|EventActorBeginOverlap
  (params (OtherActor :type Actor%20Object%20Reference)))

(event EventTick
  (params (DeltaSeconds :type Float%20%28single-precision%29)))

(event EventInteract
  (bind _particle_color_can_interact (Variables|Default|GetParticle_Color_Can_Interact))
  ;[1 1 1] On interact init animation and desactivate particle system
  (CallFunction|InitAnimation)
  (bind _alfa_track (Timeline|Desappear%20particles Play)
    (:Update
      (Effects|Components|ParticleSystem|SetColorParameter (Variables|Default|GetParticleSystem) "Fireflies_Color" (Utilities|Struct|MakeLinearColor (.r _particle_color_can_interact) (.g _particle_color_can_interact) (.b _particle_color_can_interact) _alfa_track)))))

(event EventCanInteract
  ;[1 1 1] On can interact = create new material if needed to change color and change state
  (Variables|Default|SetState "NewEnumerator1")
  (if (not (Utilities|IsValid (Variables|Default|GetDynamicMat)))
    (bind _returnvalue (Rendering|Material|CreateDynamicMaterialInstance (Variables|Default|GetSkeletalMesh) 0 "/Game/Placeable/Materials/MI_Cofre-Base.MI_Cofre-Base" "None" :!class /Script/Engine.PrimitiveComponent))
    (Variables|Default|SetDynamicMat _returnvalue)))

(event EventCannotInteract
  (Variables|Default|SetState "NewEnumerator0"))

(fn ConstructionScript)

(fn InitAnimation
  (bind _asabp_cofre (Utilities|Casting|CastToABP_Cofre (Components|SkeletalMesh|GetAnimInstance (Variables|Default|GetSkeletalMesh))))
  (Variables|/Game/Placeable/Animations/ABP_Cofre.ABP_Cofre_C|SetHas_to_Open _asabp_cofre true))

(fn UpdateMaterial
  (bind _distance (Utilities|GetNormalicedPlayerDistance))
  ;[1 1 1] Set distance to 1 if >
  (if (> _distance 1.0)
    (LocalVariables|SetDesaturation 1.0)
    (else
      (LocalVariables|SetDesaturation _distance)))
  (Rendering|Material|SetScalarParameterValue (Variables|Default|GetDynamicMat) "Desaturation" (LocalVariables|GetDesaturation) :!class /Script/Engine.MaterialInstanceDynamic))

(fn UpdateParticlesColor
  (params (Color%200 :type Linear%20Color%20Structure) (Color%201 :type Linear%20Color%20Structure))
  (Effects|Components|ParticleSystem|SetColorParameter (Variables|Default|GetParticleSystem) "Fireflies_Color" (Math|Color|Lerp(LinearColor) Color%200 Color%201 (Utilities|GetNormalicedPlayerDistance))))