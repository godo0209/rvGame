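; BP_Cofre is a placeable chest that regains its color once it becomes interactable and opens when interacted with.
; The CanInteract event creates a dynamic material instance on the skeletal mesh, and Tick then lowers its Desaturation parameter by a fixed per-frame step while above zero.
; Interact sets HasToOpen on the ABP_Cofre animation Blueprint to trigger opening and hides the particle system.
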(event EventBeginPlay)

(event Collision|EventActorBeginOverlap
  (params (OtherActor :type Actor%20Object%20Reference)))

(event EventTick
  (params (DeltaSeconds :type Float%20%28single-precision%29))
  (if (and (Variables|Default|GetCan_Interact?) (> (Variables|Default|GetDesaturation) 0.0))
    (bind _output_get (Variables|Default|SetDesaturation (- (Variables|Default|GetDesaturation) 0.01)))
    (Rendering|Material|SetScalarParameterValue (Variables|Default|GetDynamicMat) "Desaturation" _output_get :!class /Script/Engine.MaterialInstanceDynamic)))

(event EventCanInteract
  ;[1 1 1] Create new material
  (Variables|Default|SetCan_Interact? true)
  (bind _returnvalue (Rendering|Material|CreateDynamicMaterialInstance (Variables|Default|GetSkeletalMesh) 0 "/Game/Placeable/Materials/MI_Cofre-Base.MI_Cofre-Base" "None" :!class /Script/Engine.PrimitiveComponent))
  (Variables|Default|SetDynamicMat _returnvalue))

(event EventInteract
  ;[1 1 1] On interact init animation and desactivate particle system
  (CallFunction|InitAnimation)
  (Rendering|SetVisibility (Variables|Default|GetParticleSystem) false false))

(fn ConstructionScript)

(fn InitAnimation
  (bind _asabp_cofre (Utilities|Casting|CastToABP_Cofre (Components|SkeletalMesh|GetAnimInstance (Variables|Default|GetSkeletalMesh))))
  (Variables|/Game/Placeable/Animations/ABP_Cofre.ABP_Cofre_C|SetHas_to_Open _asabp_cofre true))