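; Hammer weapon Blueprint that extends a parent weapon's spawn, use and ready logic, with a glow driven by a dynamic material.
; Starting use switches the mesh to a collision channel that can break things, while Using steps up light intensity to a cap.
; Stopping restores normal collision and plays a timeline on the glow, whose update triggers the cooldown before ReadyToUse.
; When ready, the mesh moves forward for non-VR players.
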(event EventBeginPlay
  (bind _returnvalue (Rendering|Material|CreateDynamicMaterialInstance (Variables|Default|GetStaticMesh1) 0 "/Game/Placeable/Materials/Weapons/MI_Weapon-Hammer-Active.MI_Weapon-Hammer-Active" "None" :!class /Script/Engine.PrimitiveComponent))
  (Variables|Default|SetDynamic%20Mat _returnvalue))

(event Collision|EventActorBeginOverlap
  (params (OtherActor :type Actor%20Object%20Reference))
  (|CallParentFunction OtherActor) ; This node is disabled and will not be called.\nDrag off pins to build functionality.
)

(event EventTick
  (params (DeltaSeconds :type Float%20%28single-precision%29)))

(event EventSpawn
  (params (Location :type Vector :default "0, 0, 0") (Niagara%20System :type Niagara%20Component%20Object%20Reference) (Child%20Actor :type Actor%20Object%20Reference))
  (|CallParentFunction Location (Variables|Default|GetSpawn%20Weapon%20Effect) self))

(event EventReadytoUse
  (|CallParentFunction)
  (bind _asbp_character (Utilities|Casting|CastToBP_Character (Game|Player|GetPlayerPawn 0)))
  (if (not (Variables|/Game/Characters/BP_Character.BP_Character_C|GetPlaying_VR? _asbp_character))
    ;[1 1 1] To move it forward in pc
    (Transformation|SetRelativeLocation (Variables|Default|GetStaticMesh) (Variables|Default|GetOffset) false false)))

(event EventStopUsing
  (if (Utilities|Enum|Equal(Enum) (Variables|Default|GetState) "NewEnumerator3")
    (|CallParentFunction)
    ;[1 1 1] Cannot break
    (Collision|SetCollisionObjectType (Variables|Default|GetStaticMesh) "ECC_WorldDynamic")
    ;[1 1 1] Reset vfx
    (bind _returnvalue (Rendering|Material|GetScalarParameterValue (Variables|Default|GetDynamic%20Mat) "Light Intensity" :!class /Script/Engine.MaterialInstanceDynamic))
    (Variables|Default|SetCurrent%20Light%20Intensity _returnvalue)
    (bind _light_intensity (Timeline|Light%20intensity PlayFromStart)
      (:Update
        (Rendering|Material|SetScalarParameterValue (Variables|Default|GetDynamic%20Mat) "Light Intensity" _light_intensity :!class /Script/Engine.MaterialInstanceDynamic)
        (Variables|Default|SetCurrent%20Light%20Intensity (Variables|Default|GetInit%20Light%20Intensity))
        ;[1 1 1] Set ready when cd finished
        (Utilities|FlowControl|Delay (Variables|Default|GetCd))
        (CallFunction|ReadytoUse)))))

(event EventStartUsing
  (if (Utilities|Enum|Equal(Enum) (Variables|Default|GetState) "NewEnumerator5")
    (|CallParentFunction)
    ;[1 1 1] Can break
    (Collision|SetCollisionObjectType (Variables|Default|GetStaticMesh) "ECC_GameTraceChannel6")))

(fn ConstructionScript
  (|CallParentFunction))

(fn Init
  (params (Child%20Actor :type Actor%20Object%20Reference))
  (|CallParentFunction self))

(fn GetHandtoUse
  (return (Variables|Default|GetConcrete%20Hand%20To%20Use)))

(fn Using
  (if (< (Variables|Default|GetCurrent%20Light%20Intensity) (Variables|Default|GetMax%20Light%20Intensity))
    (Variables|Default|SetCurrent%20Light%20Intensity (+ (Variables|Default|GetCurrent%20Light%20Intensity) 0.5))
    (Rendering|Material|SetScalarParameterValue (Variables|Default|GetDynamic%20Mat) "Light Intensity" (Variables|Default|GetCurrent%20Light%20Intensity) :!class /Script/Engine.MaterialInstanceDynamic)))