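; Placeable shield weapon Blueprint that builds on a parent weapon class for initialization, use, spawning and readiness.
; Spawn hands its Niagara system and itself to the parent, and BeginPlay sets the explosion zone to its minimum scale.
; When ready to use outside VR, it offsets the static mesh so the shield sits forward on PC.
; It also reports which hand holds it through a configured hand value.
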(event EventBeginPlay
  (Transformation|SetRelativeScale3D (Variables|Default|GetExplosionZone) (Math|Conversions|ToVector(Float) (Variables|Default|GetMin%20Explosion%20Scale))))

(event Collision|EventActorBeginOverlap
  (params (OtherActor :type Actor%20Object%20Reference))
  (|CallParentFunction OtherActor) ; This node is disabled and will not be called.\nDrag off pins to build functionality.
)

(event EventTick
  (params (DeltaSeconds :type Float%20%28single-precision%29))
  (|CallParentFunction DeltaSeconds) ; This node is disabled and will not be called.\nDrag off pins to build functionality.
)

(event EventReadytoUse
  (|CallParentFunction)
  (bind _asbp_character (Utilities|Casting|CastToBP_Character (Game|Player|GetPlayerPawn 0)))
  (if (not (Variables|/Game/Characters/BP_Character.BP_Character_C|GetPlaying_VR? _asbp_character))
    ;[1 1 1] To move it forward in pc
    (Transformation|SetRelativeLocation (Variables|Default|GetStaticMesh) (Variables|Default|GetOffset) false false)))

(event EventStopUsing
  (|CallParentFunction))

(event EventSpawn
  (params (Location :type Vector :default "0, 0, 0") (Niagara%20System :type Niagara%20Component%20Object%20Reference) (Child%20Actor :type Actor%20Object%20Reference))
  (|CallParentFunction Location (Variables|Default|GetNiagara) self))

(event EventStartUsing
  (|CallParentFunction))

(fn ConstructionScript
  (|CallParentFunction))

(fn Init
  (params (Child%20Actor :type Actor%20Object%20Reference))
  (|CallParentFunction self))

(fn GetHandtoUse
  (return (Variables|Default|GetConcrete%20Hand%20To%20Use)))